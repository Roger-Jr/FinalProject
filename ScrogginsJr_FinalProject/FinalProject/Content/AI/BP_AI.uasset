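; BP_AI is an AI-controlled melee combatant that can attack pawns and take damage.
; Its Attack event plays a push-shove montage, and any montage notify triggers a short forward sphere trace against pawns, with debug drawing, that damages the actor hit.
; Incoming damage reduces Health, and once it is depleted the mesh switches to physics simulation as a ragdoll-style death.
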(event `self.ReceiveAnyDamage`
  (params (Damage :type "Float (single-precision)") (DamageType :type "DamageType Object Reference") (InstigatedBy :type "Controller Object Reference") (DamageCauser :type "Actor Object Reference"))
  (set `self.Health` (- (`self.Health`) Damage))
  (if (<= (`self.Health`) 0.0)
    (`PrimitiveComponent.SetSimulatePhysics` (`self.Mesh`) true)))

(event `/Game/AI/BPI_AI.Attack`
  (bind _returnvalue (`self.K2_GetActorLocation`))
  (`|PlayMontage` (`self.Mesh`) "/Game/Characters/Mannequins/Animations/Paired_PushShove_Att_Montage.Paired_PushShove_Att_Montage"
    (:`OnNotifyBegin`
      (bind (_outhit _returnvalue_2) (`KismetSystemLibrary.SphereTraceSingleForObjects` :`Start` _returnvalue :`End` (+ _returnvalue (* (`KismetMathLibrary.GetForwardVector` (`self.K2_GetActorRotation`)) 170.0)) :`Radius` 30.0 :`ObjectTypes` (`|MakeArray` "ObjectTypeQuery3" :!type "EObjectTypeQuery Enum") :`DrawDebugType` "ForDuration"))
      (if _returnvalue_2
        (`GameplayStatics.ApplyDamage` (`.HitActor` (`GameplayStatics.BreakHitResult` _outhit)) 10.0)))))

(fn `UserConstructionScript`)