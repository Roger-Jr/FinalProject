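; Ammo pickup actor that adds a fixed amount to the first-person character's TotalAmmo and then destroys itself.
; The Box overlap event casts player 0's character without checking which actor overlapped.
; The following TotalAmmo branch is redundant, as both paths destroy the pickup and print a debug string, with no cap applied.
; An unconnected older chain that clamps Ammo remains in the graph but never runs.
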(event `self.Box.OnComponentBeginOverlap`
  (params (OverlappedComponent :type "PrimitiveComponent Object Reference") (OtherActor :type "Actor Object Reference") (OtherComp :type "PrimitiveComponent Object Reference") (OtherBodyIndex :type Integer) (bFromSweep :type Boolean) (SweepResult :type "HitResult Structure (by ref)"))
  (bind _asbp_first_person_character (cast `/Game/FirstPerson/Blueprints/BP_FirstPersonCharacter` (`GameplayStatics.GetPlayerCharacter` 0)))
  (set `/Game/FirstPerson/Blueprints/BP_FirstPersonCharacter.TotalAmmo` (+ (`/Game/FirstPerson/Blueprints/BP_FirstPersonCharacter.TotalAmmo` _asbp_first_person_character) 10) _asbp_first_person_character)
  (if (>= (`/Game/FirstPerson/Blueprints/BP_FirstPersonCharacter.TotalAmmo` _asbp_first_person_character) 10)
    (`self.K2_DestroyActor`)
    (`KismetSystemLibrary.PrintString` "Hello")
    (else
      (`self.K2_DestroyActor`)
      (`KismetSystemLibrary.PrintString` "Hello"))))

(fn `UserConstructionScript`)